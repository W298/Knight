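; Player knight character with mouse-aimed facing, sprint, directional dash, blocking and melee attacks.
; Tick turns control yaw toward the cursor's ground point and derives walk speed from interpolated input axes.
; Hold/short, cooldown and switch-gate macros split attack input into light or heavy, then delayed hits strike knights tracked by AttackArea overlaps.
; Hit interpolates the victim backwards while briefly disabling input; dash only signals the AnimBP.
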(event `self.ReceiveBeginPlay`
  (bind _asknight_player_anim_bp (cast `/Game/Player/Blueprint/KnightPlayer_AnimBP` (`SkeletalMeshComponent.GetAnimInstance` (`self.Mesh`))))
  (set `self.AnimBP` _asknight_player_anim_bp))

(event `self.ReceiveTick`
  (params (DeltaSeconds :type "Float (single-precision)"))
  (`self.SetRotation`)
  (`self.SetPlayerSpeed`)
  (if (`self.isGoingBack`)
    (`self.K2_SetActorLocation` (`KismetMathLibrary.VInterpTo` (`self.K2_GetActorLocation`) (`self.BackTargetLoc`) DeltaSeconds 2.0))
    (if (== (`self.K2_GetActorLocation`) (`self.BackTargetLoc`) :`ErrorTolerance` 0.1)
      (set `self.isGoingBack` false))))

(event `Hit`
  (set `self.isGoingBack` true)
  (set `self.BackTargetLoc` (+ (`self.K2_GetActorLocation`) (* (`self.GetActorForwardVector`) -200)))
  (set `self.followMouse` false)
  (`self.DisableInput` null)
  (set `self.Action` "NewEnumerator5")
  (`KismetSystemLibrary.Delay` 0.2)
  (set `self.Action` "NewEnumerator6")
  (`KismetSystemLibrary.Delay` 1.0)
  (`self.EnableInput` null)
  (set `self.followMouse` true))

(event `InputAction|Debug`
  (params (Key :type "Key Structure"))
  (:`Pressed`
    (`self.Hit`)))

(event `ApplyAttack`
  (for _array_element (`self.AttackableActors`)
    (if (!= _array_element self)
      (bind _asknight_player (cast `/Game/Player/Blueprint/KnightPlayer` _array_element))
      (`self.Hit` _asknight_player))))

(event `self.AttackArea.OnComponentBeginOverlap`
  (params (OverlappedComponent :type "PrimitiveComponent Object Reference") (OtherActor :type "Actor Object Reference") (OtherComp :type "PrimitiveComponent Object Reference") (OtherBodyIndex :type Integer) (bFromSweep :type Boolean) (SweepResult :type "HitResult Structure (by ref)"))
  (`KismetArrayLibrary.Array_AddUnique` (`self.AttackableActors`) OtherActor))

(event `self.AttackArea.OnComponentEndOverlap`
  (params (OverlappedComponent :type "PrimitiveComponent Object Reference") (OtherActor :type "Actor Object Reference") (OtherComp :type "PrimitiveComponent Object Reference") (OtherBodyIndex :type Integer))
  (`KismetArrayLibrary.Array_RemoveItem` (`self.AttackableActors`) OtherActor))

(event `InputAction|Dash`
  (params (Key :type "Key Structure"))
  (bind _returnvalue (`self.GetInputAxisValue`))
  (bind _returnvalue_2 (`self.GetInputAxisValue`))
  (bind _animbp (`self.AnimBP`))
  (bind _animbp_2 (`self.AnimBP`))
  (:`Pressed`
    (if (!= _returnvalue 0.0)
      (if (< _returnvalue 0.0)
        (set `/Game/Player/Blueprint/KnightPlayer_AnimBP.dashDirection` "NewEnumerator1" _animbp_2)
        (else
          (set `/Game/Player/Blueprint/KnightPlayer_AnimBP.dashDirection` "NewEnumerator0" _animbp_2)))
      (`KismetSystemLibrary.Delay` 0.05 :!label _label)
      (set `/Game/Player/Blueprint/KnightPlayer_AnimBP.dashDirection` "NewEnumerator4" (`self.AnimBP`))
      (elif (!= _returnvalue_2 0.0)
        (if (< _returnvalue_2 0.0)
          (set `/Game/Player/Blueprint/KnightPlayer_AnimBP.dashDirection` "NewEnumerator3" _animbp)
          (goto _label)
          (else
            (set `/Game/Player/Blueprint/KnightPlayer_AnimBP.dashDirection` "NewEnumerator2" _animbp)
            (goto _label)))))))

(event `InputAction|Block`
  (params (Key :type "Key Structure"))
  (:`Pressed`
    (set `self.isBlocking` true))
  (:`Released`
    (set `self.isBlocking` false)))

(event `InputAction|BasicAttack`
  (params (Key :type "Key Structure"))
  (:`Pressed`
    (`self.Hold / Short` 0.2 :!label _label_2
      (:`Short`
        (`self.Press / Release CoolDown` :!label _label_3
          (:`Pressed Out`
            (set `self.attack` true)
            (`KismetSystemLibrary.Delay` 0.35)
            (`self.ApplyAttack` :!label _label_4))
          (:`Released Out`
            (set `self.attack` false))))
      (:`Short Released`
        (goto _label_3 :!via `Released`))
      (:`Holding`
        (set `self.heavyattack` true)
        (`KismetSystemLibrary.Delay` 0.7)
        (goto _label_4))
      (:`Holding Released`
        (set `self.heavyattack` false))))
  (:`Released`
    (goto _label_2 :!via `Released`)))

(event `InputAction|Sprint`
  (params (Key :type "Key Structure"))
  (:`Pressed`
    (set `self.MaxAxisV` 1.0)
    (set `self.isSprinting` true))
  (:`Released`
    (set `self.MaxAxisV` 0.5)
    (set `self.isSprinting` false)))

(event `InputAxis|MoveRight`
  (params (AxisValue :type "Float (single-precision)"))
  (set `self.RightAxisV` (`KismetMathLibrary.FInterpTo` (`self.RightAxisV`) (`KismetMathLibrary.FClamp` AxisValue (* -1 (`self.MaxAxisV`)) (`self.MaxAxisV`)) (`GameplayStatics.GetWorldDeltaSeconds`) 4.0)))

(event `InputAxis|MoveForward`
  (params (AxisValue :type "Float (single-precision)"))
  (set `self.ForwardAxisV` (`KismetMathLibrary.FInterpTo` (`self.ForwardAxisV`) (`KismetMathLibrary.FClamp` AxisValue (* -1 (`self.MaxAxisV`)) (`self.MaxAxisV`)) (`GameplayStatics.GetWorldDeltaSeconds`) 4.0)))

(fn `GetMousePosOnWorld`
  (params (Z :type "Float (double-precision)"))
  (returns (Position :type "Vector Structure"))
  (bind (_worldlocation _worlddirection) (`PlayerController.DeprojectMousePositionToWorld` (`GameplayStatics.GetPlayerController` 0)))
  (return (+ (+ _worldlocation (* (* _worlddirection (/ (.z _worldlocation) (.z _worlddirection))) -1.0)) (`KismetMathLibrary.MakeVector` 0.0 0.0 Z))))

(fn `SetPlayerSpeed`
  (set `CharacterMovementComponent.MaxWalkSpeed` (`KismetMathLibrary.MapRangeUnclamped` (`KismetMathLibrary.Sqrt` (+ (`KismetMathLibrary.Square` (`self.ForwardAxisV`)) (`KismetMathLibrary.Square` (`self.RightAxisV`)))) 0.0 1.414 0.0 440.0) (`self.CharacterMovement`)))

(fn `SetRotation`
  (if (`self.followMouse`)
    (bind _position (`self.GetMousePosOnWorld` 0.0))
    (if (not (`self.isEquipping`))
      (bind (_returnvalue_roll _returnvalue_pitch _returnvalue_yaw) (`KismetMathLibrary.BreakRotator` (`KismetMathLibrary.FindLookAtRotation` (`self.K2_GetActorLocation`) _position)))
      (`Controller.SetControlRotation` (`GameplayStatics.GetPlayerController` 0) (`KismetMathLibrary.MakeRotator` 0.0 0.0 _returnvalue_yaw))))
  (return))

(fn `UserConstructionScript`)