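; Knight player Blueprint that turns input into movement values and attack flags, and yaws the controller toward the cursor's hit point each tick unless equipping.
; Each direction key drives a timeline-based ease macro that writes its own Forward, Backward, Right or Left value.
; A Hold/Short macro uses a brief delay to split BasicAttack into a tap, which sets Attack through a press cooldown, or a hold, which sets Heavyattack.
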(event `InputAction|ForwardKey`
  (params (Key :type "Key Structure"))
  (:`Pressed`
    (`/Engine/EditorBlueprintResources/StandardMacros.Gate` false :!label _label
      (:`Exit`
        (`/Engine/EditorBlueprintResources/StandardMacros.DoOnce` false :!label _label_2
          (:`Completed`
            (bind (_direction _axisvalue) (`Timeline|Ease` :!via `PlayFromStart` :!label _label_3)
              (:`Update`
                (set `self.ForwardV` _axisvalue))))))))
  (:`Released`
    (`|ExecutionSequence`
      (:`then_0`
        (goto _label_2 :!via `Reset`))
      (:`then_1`
        (goto _label :!via `Open`))
      (:`then_2`
        (goto _label_3 :!via `ReverseFromEnd`)))))

(event `self.ReceiveTick`
  (params (DeltaSeconds :type "Float (single-precision)"))
  (bind _returnvalue (`GameplayStatics.GetPlayerController` null))
  (bind (_returnvalue_x _returnvalue_y) (`KismetMathLibrary.BreakVector` (- (`.Location` (`GameplayStatics.BreakHitResult` (`PlayerController.GetHitResultUnderCursorByChannel` _returnvalue "TraceTypeQuery1" true))) (`Actor.K2_GetActorLocation`))))
  (bind (_returnvalue_roll _returnvalue_pitch _returnvalue_yaw) (`KismetMathLibrary.BreakRotator` (`KismetMathLibrary.FindLookAtRotation` (`Actor.GetActorForwardVector`) (`KismetMathLibrary.MakeVector` _returnvalue_x _returnvalue_y))))
  (cast `` (`GameplayStatics.GetGameMode` null))
  (if (not (`self.isEquipping`))
    (`Controller.SetControlRotation` _returnvalue (`KismetMathLibrary.MakeRotator` 0.0 0.0 _returnvalue_yaw))))

(event `InputAction|BackwardKey`
  (params (Key :type "Key Structure"))
  (:`Pressed`
    (`/Engine/EditorBlueprintResources/StandardMacros.Gate` false :!label _label_4
      (:`Exit`
        (`/Engine/EditorBlueprintResources/StandardMacros.DoOnce` false :!label _label_5
          (:`Completed`
            (bind (_direction _axisvalue) (`Timeline|타임라인_0` :!via `PlayFromStart` :!label _label_6)
              (:`Update`
                (set `self.BackwardV` _axisvalue))))))))
  (:`Released`
    (`|ExecutionSequence`
      (:`then_0`
        (goto _label_5 :!via `Reset`))
      (:`then_1`
        (goto _label_4 :!via `Open`))
      (:`then_2`
        (goto _label_6 :!via `ReverseFromEnd`)))))

(event `InputAction|RightKey`
  (params (Key :type "Key Structure"))
  (:`Pressed`
    (`/Engine/EditorBlueprintResources/StandardMacros.Gate` false :!label _label_7
      (:`Exit`
        (`/Engine/EditorBlueprintResources/StandardMacros.DoOnce` false :!label _label_8
          (:`Completed`
            (bind (_direction _axisvalue) (`Timeline|타임라인_1` :!via `PlayFromStart` :!label _label_9)
              (:`Update`
                (set `self.RightV` _axisvalue))))))))
  (:`Released`
    (`|ExecutionSequence`
      (:`then_0`
        (goto _label_8 :!via `Reset`))
      (:`then_1`
        (goto _label_7 :!via `Open`))
      (:`then_2`
        (goto _label_9 :!via `ReverseFromEnd`)))))

(event `InputAction|LeftKey`
  (params (Key :type "Key Structure"))
  (:`Pressed`
    (`/Engine/EditorBlueprintResources/StandardMacros.Gate` false :!label _label_10
      (:`Exit`
        (`/Engine/EditorBlueprintResources/StandardMacros.DoOnce` false :!label _label_11
          (:`Completed`
            (bind (_direction _axisvalue) (`Timeline|타임라인_2` :!via `PlayFromStart` :!label _label_12)
              (:`Update`
                (set `self.LeftV` _axisvalue))))))))
  (:`Released`
    (`|ExecutionSequence`
      (:`then_0`
        (goto _label_11 :!via `Reset`))
      (:`then_1`
        (goto _label_10 :!via `Open`))
      (:`then_2`
        (goto _label_12 :!via `ReverseFromEnd`)))))

(event `InputAction|BasicAttack`
  (params (Key :type "Key Structure"))
  (:`Pressed`
    (`self.Hold / Short` :!label _label_13
      (:`Short`
        (`self.Press / Release CoolDown` :!label _label_14
          (:`PressOut`
            (set `self.attack` true))
          (:`ReleaseOut`
            (set `self.attack` false))))
      (:`Holding`
        (set `self.heavyattack` true))
      (:`Short Released`
        (goto _label_14 :!via `Released`))
      (:`Holding Released`
        (set `self.heavyattack` false))))
  (:`Released`
    (goto _label_13 :!via `Released`)))

(fn `UserConstructionScript`)